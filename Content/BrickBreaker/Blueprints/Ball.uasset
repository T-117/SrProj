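; Brick breaker ball that launches with physics velocity and has its speed capped on impact.
; It enables player input on begin play, and pressing L fires it along world +X, then disables input so it launches only once.
; On each hit, it clamps the hit component's linear velocity to the FloatingPawnMovement max speed, using that component as a speed setting for the physics body.
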(event `self.ReceiveBeginPlay`
  (`self.EnableInput` (`GameplayStatics.GetPlayerController` 0)))

(event `Key|L`
  (params (Key :type "Key Structure" :default "AnyKey"))
  (:`Pressed`
    (`PrimitiveComponent.SetPhysicsLinearVelocity` (`self.Ball`) (1000.0 0.0 0.0) false "None")
    (`self.DisableInput` (`GameplayStatics.GetPlayerController` 0))))

(event `self.ReceiveHit`
  (params (MyComp :type "PrimitiveComponent Object Reference") (Other :type "Actor Object Reference") (OtherComp :type "PrimitiveComponent Object Reference") (bSelfMoved :type Boolean) (HitLocation :type "Vector Structure") (HitNormal :type "Vector Structure") (NormalImpulse :type "Vector Structure") (Hit :type "HitResult Structure (by ref)"))
  ;[1 1 1] Clamp Ball velocity
  (bind _returnvalue (`PrimitiveComponent.GetPhysicsLinearVelocity` MyComp "None"))
  (`PrimitiveComponent.SetPhysicsLinearVelocity` MyComp (`KismetMathLibrary.ClampVectorSize` _returnvalue 0.0 (`MovementComponent.GetMaxSpeed` (`self.FloatingPawnMovement`))) false "None"))

(fn `UserConstructionScript`)