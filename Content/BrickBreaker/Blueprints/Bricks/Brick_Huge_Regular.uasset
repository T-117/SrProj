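; Huge regular brick for the brick breaker game that breaks into medium bricks when destroyed.
; Construction scales the inherited health by the tough toughness multiplier and the face size by the mesh's world scale.
; The Destruction event removes the mesh, then spawns eight Brick_Medium_Regular actors at the octant centers, found by skipping zero indices in a triple loop.
; Offsets follow the brick's rotation, but spawned bricks get zero rotation.
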(event `self.ReceiveBeginPlay`)

(event `self.ReceiveActorBeginOverlap`
  (params (OtherActor :type "Actor Object Reference")))

(event `self.ReceiveTick`
  (params (DeltaSeconds :type "Float (single-precision)")))

(event `self.Destruction`
  (`self.BrickDestruction`))

(fn `BrickDestruction`
  (bind _staticmesh (`self.StaticMesh`))
  (bind _returnvalue (/ (`self.FaceSize`) 4.0))
  (set `self.location` (`SceneComponent.K2_GetComponentLocation` _staticmesh))
  (set `self.rotation` (`SceneComponent.K2_GetComponentRotation` _staticmesh))
  (`ActorComponent.K2_DestroyComponent` (`self.StaticMesh`))
  (for _index (range -1 2)
    (for _index_2 (range -1 2)
      (for _index_3 (range -1 2)
        (if (not (== (* _index_3 _index_2 _index) 0))
          (`|SpawnActorFromClass` "/Game/BrickBreaker/Blueprints/Bricks/Brick_Medium_Regular.Brick_Medium_Regular_C" (`KismetMathLibrary.MakeTransform` (+ (`self.location`) (`KismetMathLibrary.GreaterGreater_VectorRotator` (`KismetMathLibrary.MakeVector` (* _index_3 _returnvalue) (* _index_2 _returnvalue) (* _index _returnvalue)) (`self.rotation`)))) "AdjustIfPossibleButAlwaysSpawn" "OverrideRootScale")))))
  (`self.K2_DestroyActor`)
  (return))

(fn `UserConstructionScript`
  (`parent.UserConstructionScript`)
  (set `self.Health` (* (`self.Health`) (`self.Toughness_Tough`)))
  (set `self.FaceSize` (* (`self.FaceSize`) (.x (`SceneComponent.K2_GetComponentScale` (`self.StaticMesh`))))))