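; Brick_Small_Regular is a small brick variant for the BrickBreaker game, built as a child brick Blueprint.
; Its construction script runs the parent script, then sets Health from BaseHealth scaled by the tough toughness multiplier.
; It also derives FaceSize from BaseFaceSize and the brick mesh's world X scale.
; The event graph holds only disabled placeholder events, so it adds no runtime logic.
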(event `self.ReceiveBeginPlay`)

(event `self.ReceiveActorBeginOverlap`
  (params (OtherActor :type "Actor Object Reference")))

(event `self.ReceiveTick`
  (params (DeltaSeconds :type "Float (single-precision)")))

(fn `UserConstructionScript`
  (`parent.UserConstructionScript`)
  (set `self.Health` (* (`self.BaseHealth`) (`self.Toughness_Tough`)))
  (set `self.FaceSize` (* (`self.BaseFaceSize`) (.x (`SceneComponent.K2_GetComponentScale` (`self.BrickMesh`))))))