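; Medium weak brick for a brick-breaker game that shatters into eight small weak bricks when destroyed.
; Construction derives health from the ToughnessTough multiplier and face size from the mesh's world scale.
; The Destruction event removes the mesh, spawns dust, then uses nested loops that skip zero indices to place small bricks at the cube's rotated corner offsets before destroying the actor.
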(event `self.ReceiveBeginPlay`)

(event `self.ReceiveActorBeginOverlap`
  (params (OtherActor :type "Actor Object Reference")))

(event `self.ReceiveTick`
  (params (DeltaSeconds :type "Float (single-precision)")))

(event `self.Destruction`
  (`self.BrickDestruction`))

(fn `BrickDestruction`
  (bind _brickmesh (`self.BrickMesh`))
  (bind _returnvalue (/ (`self.FaceSize`) 4.0))
  (set `self.location` (`SceneComponent.K2_GetComponentLocation` _brickmesh))
  (set `self.rotation` (`SceneComponent.K2_GetComponentRotation` _brickmesh))
  (`ActorComponent.K2_DestroyComponent` (`self.BrickMesh`))
  (`|SpawnActorFromClass` "/Game/BrickBreaker/Blueprints/BrickDust.BrickDust_C" (`KismetMathLibrary.MakeTransform` (`self.location`) (struct) (1.0 1.0 1.0)) "AlwaysSpawn" "OverrideRootScale")
  (for _index (range -1 2)
    (for _index_2 (range -1 2)
      (for _index_3 (range -1 2)
        (if (not (== (* _index_3 _index_2 _index) 0))
          (`|SpawnActorFromClass` "/Game/BrickBreaker/Blueprints/Bricks/Brick_Small_Weak.Brick_Small_Weak_C" (`KismetMathLibrary.MakeTransform` (+ (`self.location`) (`KismetMathLibrary.GreaterGreater_VectorRotator` (`KismetMathLibrary.MakeVector` (* _index_3 _returnvalue) (* _index_2 _returnvalue) (* _index _returnvalue)) (`self.rotation`)))) "AdjustIfPossibleButAlwaysSpawn" "OverrideRootScale")))))
  (`self.K2_DestroyActor`)
  (return))

(fn `UserConstructionScript`
  (`parent.UserConstructionScript`)
  (set `self.Health` (* (`self.BaseHealth`) (`self.Toughness_Tough`)))
  (set `self.FaceSize` (* (`self.BaseFaceSize`) (.x (`SceneComponent.K2_GetComponentScale` (`self.BrickMesh`))))))