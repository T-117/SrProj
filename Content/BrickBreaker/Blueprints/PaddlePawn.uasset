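; PaddlePawn is the player-controlled paddle for the brick breaker game.
; MoveUp and MoveRight share one swept SetActorLocation, scaled by max speed and delta time, that adds the axis value to both Y and Z.
; MouseX and MouseY likewise share one camera rotation applied to both pitch and yaw.
; On BeginPlay, it spawns a Ball slightly offset along X from the paddle.
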(event `InputAxisKey|MouseY`
  (params (AxisValue :type "Float (single-precision)"))
  ;[1 1 1] Camera Rotation controls
  (`SceneComponent.K2_AddRelativeRotation` (`self.Camera`) (`KismetMathLibrary.MakeRotator` 0.0 AxisValue (stale `InputAxisKey|MouseX` AxisValue)) true false :!label _label))

(event `InputAxisKey|MouseX`
  (params (AxisValue :type "Float (single-precision)"))
  ;[1 1 1] Camera Rotation controls
  (goto _label))

(event `InputAxis|MoveUp`
  (params (AxisValue :type "Float (single-precision)"))
  (bind _returnvalue (`GameplayStatics.GetWorldDeltaSeconds`))
  (bind _returnvalue_2 (`MovementComponent.GetMaxSpeed` (`self.FloatingPawnMovement`)))
  ;[1 1 1] Paddle Movement controls
  (`self.K2_SetActorLocation` (`KismetMathLibrary.MakeVector` (.x (`self.K2_GetActorLocation`)) (+ (.y (`self.K2_GetActorLocation`)) (* (stale `InputAxis|MoveRight` AxisValue) _returnvalue _returnvalue_2)) (+ (.z (`self.K2_GetActorLocation`)) (* AxisValue _returnvalue _returnvalue_2))) true :!label _label_2))

(event `InputAxis|MoveRight`
  (params (AxisValue :type "Float (single-precision)"))
  ;[1 1 1] Paddle Movement controls
  (goto _label_2))

(event `self.ReceiveBeginPlay`
  (`self.SpawnBallOntoPaddle`))

(fn `SpawnBallOntoPaddle`
  (`|SpawnActorFromClass` "/Game/BrickBreaker/Blueprints/Ball.Ball_C" (`KismetMathLibrary.MakeTransform` (`KismetMathLibrary.MakeVector` (+ (.x (`SceneComponent.K2_GetComponentLocation` (`self.Paddle`))) 65.0) (.y (`SceneComponent.K2_GetComponentLocation` (`self.Paddle`))) (.z (`SceneComponent.K2_GetComponentLocation` (`self.Paddle`))))) "AlwaysSpawn" "OverrideRootScale")
  (return))

(fn `UserConstructionScript`)