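; Brick Breaker volume actor that spawns an A_BrickBase brick each time the M key is pressed.
; It picks a random point within the SpawnBox's scaled extents, offset from the actor's location along world axes, and applies a random rotation including roll.
; Spawning nudges the brick clear of collisions and skips it if no free spot is found.
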(event `self.ReceiveBeginPlay`)

(event `self.ReceiveActorBeginOverlap`
  (params (OtherActor :type "Actor Object Reference")))

(event `self.ReceiveTick`
  (params (DeltaSeconds :type "Float (single-precision)")))

(event `Key|M`
  (params (Key :type "Key Structure" :default "AnyKey"))
  (bind _x (.x (`BoxComponent.GetScaledBoxExtent` (`self.SpawnBox`))))
  (bind _y (.y (`BoxComponent.GetScaledBoxExtent` (`self.SpawnBox`))))
  (bind _z (.z (`BoxComponent.GetScaledBoxExtent` (`self.SpawnBox`))))
  (:`Pressed`
    (`|SpawnActorFromClass` "/Game/BrickBreaker/Blueprints/A_BrickBase.A_BrickBase_C" (`KismetMathLibrary.MakeTransform` (+ (`KismetMathLibrary.MakeVector` (`KismetMathLibrary.RandomFloatInRange` (* _x -1.0) _x) (`KismetMathLibrary.RandomFloatInRange` (* _y -1.0) _y) (`KismetMathLibrary.RandomFloatInRange` (* _z -1.0) _z)) (`self.K2_GetActorLocation`)) (`KismetMathLibrary.RandomRotator` true)) "AdjustIfPossibleButDontSpawnIfColliding" "OverrideRootScale")))

(fn `UserConstructionScript`)